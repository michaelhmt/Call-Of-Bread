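; Drawer actor that slides open and closed along the Y axis, toggled by a triggerable event.
; The DrawerMovement timeline plays or reverses based on IsClosed, offsetting the actor's relative location from the world location cached at BeginPlay.
; BeginPlay inverts the flag and runs the toggle once to apply the configured starting state.
; TriggerableEvent toggles after its Delay, ignoring SwitchState and Value.
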(event Custom|Event%20Triggerable%20Event
  (params (Switch%20State :type Boolean) (Value :type Float%20%28single-precision%29) (Delay :type Float%20%28single-precision%29))
  (bind _initial_position (Variables|Default|GetInitial%20Position))
  (Utilities|FlowControl|Delay Delay)
  (if (Variables|Default|GetIs%20Closed)
    (Variables|Default|SetIs%20Closed false)
    (bind _block_y_position (Timeline|Drawer%20Movement Play)
      (:Update
        (Transformation|SetActorRelativeLocation (Math|Vector|MakeVector (.x _initial_position) (+ (.y _initial_position) _block_y_position) (.z _initial_position)))))
    (else
      (Variables|Default|SetIs%20Closed true)
      (Timeline|Drawer%20Movement Reverse))))

(event EventBeginPlay
  (Variables|Default|SetInitial%20Position (Transformation|GetActorLocation))
  (if (Variables|Default|GetIs%20Closed)
    (Variables|Default|SetIs%20Closed false)
    (else
      (Variables|Default|SetIs%20Closed true)))
  (if (Variables|Default|GetIs%20Closed)
    (Variables|Default|SetIs%20Closed false)
    (bind _block_y_position (Timeline|Drawer%20Movement Play)
      (:Update
        (Transformation|SetActorRelativeLocation (Math|Vector|MakeVector (.x (Variables|Default|GetInitial%20Position)) (+ (.y (Variables|Default|GetInitial%20Position)) _block_y_position) (.z (Variables|Default|GetInitial%20Position))))))
    (else
      (Variables|Default|SetIs%20Closed true)
      (Timeline|Drawer%20Movement Reverse))))

(fn ConstructionScript)