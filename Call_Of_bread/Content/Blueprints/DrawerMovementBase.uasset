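; Drawer Blueprint that slides its Drawer component open when the ThirdPersonCharacter overlaps DrawerCollision and closed when it leaves.
; The construction script stores the closed world location and an open one offset along negative world Y, regardless of rotation.
; The DrawerMove timeline plays or reverses, feeding its Movement track into VInterpTo's DeltaTime as a blend alpha between the two positions.
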(event OnComponentBeginOverlap(DrawerCollision)
  (params (OverlappedComponent :type Primitive%20Component%20Object%20Reference) (OtherActor :type Actor%20Object%20Reference) (OtherComp :type Primitive%20Component%20Object%20Reference) (OtherBodyIndex :type Integer) (bFromSweep :type Boolean) (SweepResult :type Hit%20Result%20Structure%20%28by%20ref%29))
  (Utilities|Casting|CastToThirdPersonCharacter OtherActor)
  (bind _movement (Timeline|DrawerMove Play)
    (:Update
      (Transformation|SetWorldLocation (Variables|Default|GetDrawer) (Math|Interpolation|VInterpTo (Variables|Default|GetDrawer%20Closed) (Variables|Default|GetDrawer%20Open) _movement 1.0) false false))))

(event OnComponentEndOverlap(DrawerCollision)
  (params (OverlappedComponent :type Primitive%20Component%20Object%20Reference) (OtherActor :type Actor%20Object%20Reference) (OtherComp :type Primitive%20Component%20Object%20Reference) (OtherBodyIndex :type Integer))
  (Utilities|Casting|CastToThirdPersonCharacter OtherActor)
  (bind _movement (Timeline|DrawerMove Reverse)
    (:Update
      (Transformation|SetWorldLocation (Variables|Default|GetDrawer) (Math|Interpolation|VInterpTo (Variables|Default|GetDrawer%20Closed) (Variables|Default|GetDrawer%20Open) _movement 1.0) false false))))

(fn ConstructionScript
  (bind _output_get (Variables|Default|SetDrawer%20Closed (Transformation|GetWorldLocation (Variables|Default|GetDrawer))))
  (Variables|Default|SetDrawer%20Open (Math|Vector|MakeVector (.X (Math|Vector|BreakVector _output_get)) (+ (.Y (Math|Vector|BreakVector _output_get)) -1.2e+02) (.Z (Math|Vector|BreakVector _output_get)))))